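; StateTree task that moves the AI Character to the location of a supplied TargetTriggerSphere.
; On entry it runs AI MoveTo, clears IsOk once the move starts, and finishes successfully shortly after arrival.
; An invalid target or failed move only prints debug text, leaving the task unfinished.
; ExitState is empty; disconnected leftover logic would parse the sphere's tag into BP_Berge's CurrZoneNum and set IsOk.
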(event `self.ReceiveLatentEnterState`
  (params (Transition :type "StateTreeTransitionResult Structure (by ref)"))
  (bind _targettriggersphere (`self.TargetTriggerSphere`))
  (`KismetSystemLibrary.PrintString` "Enter state....")
  (`/Engine/EditorBlueprintResources/StandardMacros.IsValid` _targettriggersphere
    (:`Is Valid`
      (`|AIMoveTo` (`self.Character`) (`Actor.K2_GetActorLocation` _targettriggersphere) null 5.0 true
        (:`then`
          (`KismetSystemLibrary.PrintString` "Movingn....")
          (set `self.IsOk` false))
        (:`OnSuccess`
          (`KismetSystemLibrary.PrintString` "ON Succe")
          (`KismetSystemLibrary.Delay` 0.2)
          (`self.FinishTask` true))
        (:`OnFail`
          (`KismetSystemLibrary.PrintString` "on fail"))))
    (:`Is Not Valid`
      (`KismetSystemLibrary.PrintString` "Not valid....."))))

(event `self.ReceiveExitState`
  (params (Transition :type "StateTreeTransitionResult Structure (by ref)")))