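; State Tree evaluator that finds the navigation point nearest to the context actor, a BP_Berge, when the tree starts.
; It gathers all TriggerSphere actors tagged NavPt, unhides them in game and picks the closest to the actor's location.
; The nearest point's name is printed, then stored on BP_Berge as both its current and target trigger sphere.
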(event `self.ReceiveTreeStart`
  (bind _outactors (`GameplayStatics.GetAllActorsOfClassWithTag` "/Script/Engine.TriggerSphere" "NavPt"))
  (bind _output_get (set `self.AllNavPts` _outactors))
  (for _array_element _output_get
    (`Actor.SetActorHiddenInGame` _array_element false))
  (bind (_distance _returnvalue) (`GameplayStatics.FindNearestActor` (`Actor.K2_GetActorLocation` (`self.CtxActor`)) _output_get))
  (bind _astrigger_sphere (cast `TriggerSphere` _returnvalue))
  (`KismetSystemLibrary.PrintString` (`KismetStringLibrary.Concat_StrStr` "The Nearest NavPt:  " (`KismetSystemLibrary.GetDisplayName` _returnvalue)))
  (bind _asbp_berge (cast `/Game/Blueprints/BP_Berge` (`self.CtxActor`)))
  (set `/Game/Blueprints/BP_Berge.CurrTriggerSphere` _astrigger_sphere _asbp_berge)
  (set `/Game/Blueprints/BP_Berge.TargetTriggerSphere` _astrigger_sphere _asbp_berge))