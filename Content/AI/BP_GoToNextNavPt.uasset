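; StateTree task that moves a BP_Berge character to its next nav point along a patrol route ordered by zone number and letter.
; It reads both from trigger-sphere tags, seeking the adjacent letter in the same zone, then the first or last point of the neighboring zone.
; Direction flips at either end of the route.
; AIMoveTo performs the move, updating the character's nav point on success and finishing the task with the result.
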(event `self.ReceiveLatentEnterState`
  (params (Transition :type "StateTreeTransitionResult Structure (by ref)"))
  (bind _chara (`self.Chara`))
  (bind _asbp_berge (cast `/Game/Blueprints/BP_Berge` (`self.CurrCharacter`)))
  (set `self.Chara` _asbp_berge)
  (bind (_foundrsl _nextnavpt) (`self.FindNextNavPt_SameZone` (`/Game/Blueprints/BP_Berge.IsGoPrevNavPt` (`self.Chara`))))
  (if _foundrsl
    (`self.MoveCharacterNow` _nextnavpt)
    (else
      (bind (_isfound _navpt) (`self.FindNavPt_NextZone` (`/Game/Blueprints/BP_Berge.IsGoPrevNavPt` (`self.Chara`))))
      (if _isfound
        (`self.MoveCharacterNow` _navpt)
        (else
          (set `/Game/Blueprints/BP_Berge.IsGoPrevNavPt` true _chara)
          (`self.MoveCharacterNow` (`/Game/Blueprints/BP_Berge.CurrTriggerSphere` _chara)))))))

(event `self.ReceiveLatentTick`
  (params (DeltaTime :type "Float (single-precision)")))

(fn `ExtraCurrNavPtNum`
  (params (NavPt :type "TriggerSphere Object Reference"))
  (returns (NavPtNum :type Integer))
  (bind _tags (`Actor.Tags` NavPt))
  (if (== (`KismetArrayLibrary.Array_Length` _tags) 3)
    (return -1)
    (else
      (return (`KismetMathLibrary.Clamp` (`KismetStringLibrary.GetCharacterAsNumber` (`KismetStringLibrary.Conv_NameToString` (`|GetArrayItem` _tags 2))) 65 90)))))

(fn `ExtraCurrNavPtNum_OneActor`
  (params (TirggerActor :type "TriggerSphere Object Reference"))
  (returns (NavPtNum :type Integer))
  (return (`KismetStringLibrary.GetCharacterAsNumber` (`KismetStringLibrary.Conv_NameToString` (`|GetArrayItem` (`Actor.Tags` TirggerActor) 2)))))

(fn `ExtraCurrNavZoneNum`
  (params (NavPt :type "TriggerSphere Object Reference"))
  (returns (ZonetNum :type Integer))
  (bind _tags (`Actor.Tags` NavPt))
  (if (== (`KismetArrayLibrary.Array_Length` _tags) 3)
    (return (`KismetStringLibrary.Conv_StringToInt` (`KismetStringLibrary.Conv_NameToString` (`|GetArrayItem` _tags 1))))
    (else
      (return -1))))

(fn `FindNavPt_NextZone`
  (params (GoPrev :type Boolean))
  (returns (IsFound :type Boolean) (NavPt :type "TriggerSphere Object Reference"))
  (locals (NextZoneNum :type Integer) (PrevZoneNum :type Integer) (TmpNavPt :type "TriggerSphere Object Reference") (NextZoneNavPts :type "Array of TriggerSphere Object Reference") (PrevZoneNavPts :type "Array of TriggerSphere Object Reference"))
  (bind _chara (`self.Chara`))
  (bind _returnvalue (+ (`self.ExtraCurrNavZoneNum` (`/Game/Blueprints/BP_Berge.TargetTriggerSphere` (`self.Chara`))) (select `bool` GoPrev :`false` 1 :`true` -1)))
  (`|ExecutionSequence`
    (:`then_0`
      (if (< _returnvalue 1)
        (set `/Game/Blueprints/BP_Berge.IsGoPrevNavPt` false _chara)
        (return true (`/Game/Blueprints/BP_Berge.CurrTriggerSphere` _chara))
        (else
          (set `local.NextZoneNum` _returnvalue)
          (for _array_element (`self.AllNavPts`)
            (bind _output_get (set `local.TmpNavPt` _array_element))
            (if (== (`self.ExtraCurrNavZoneNum` _output_get) (`local.NextZoneNum`))
              (`KismetArrayLibrary.Array_Add` (`local.NextZoneNavPts`) (`local.TmpNavPt`)))))))
    (:`then_1`
      (if (`KismetArrayLibrary.Array_IsNotEmpty` (`local.NextZoneNavPts`))
        (bind _sortednavpts (`self.SimpleSortNavPt_SameZone` (`local.NextZoneNavPts`) (`local.GoPrev`)))
        (return true (`|GetArrayItem` _sortednavpts))
        (else
          (return false null))))))

(fn `FindNextNavPt_SameZone`
  (params (FindPrev :type Boolean))
  (returns (FoundRsl :type Boolean) (NextNavPt :type "TriggerSphere Object Reference"))
  (locals (TmpTags :type "Array of Name"))
  (bind _output_get (set `local.TmpTags` (`Actor.Tags` (`/Game/Blueprints/BP_Berge.TargetTriggerSphere` (`self.Chara`)))))
  (if (== (`KismetArrayLibrary.Array_Length` _output_get) 3)
    (for _array_element (`self.AllNavPts`)
      (if (and (`Actor.ActorHasTag` _array_element (`KismetStringLibrary.Conv_StringToName` (`KismetStringLibrary.Conv_IntToString` (`self.ExtraCurrNavZoneNum` (`/Game/Blueprints/BP_Berge.TargetTriggerSphere` (`self.Chara`)))))) (== (+ (`self.ExtraCurrNavPtNum_OneActor` (`/Game/Blueprints/BP_Berge.TargetTriggerSphere` (`self.Chara`))) (select `bool` (`local.FindPrev`) :`false` 1 :`true` -1)) (`self.ExtraCurrNavPtNum_OneActor` _array_element)))
        (return true _array_element)))
    (return false null)
    (else
      (`KismetSystemLibrary.PrintString` "Please set trigger sphere tags correctly....")
      (return false null))))

(fn `SimpleSortNavPt_SameZone`
  (params (NavPts :type "Array of TriggerSphere Object Reference") (IsDescend :type Boolean))
  (returns (SortedNavPts :type "Array of TriggerSphere Object Reference"))
  (locals (TmpNavPts :type "Array of TriggerSphere Object Reference") (TmpNavPtsIn :type "Array of TriggerSphere Object Reference"))
  (bind _tmpnavptsin (`local.TmpNavPtsIn`))
  (bind _returnvalue (`KismetStringLibrary.GetCharacterAsNumber` "A"))
  (if (`KismetArrayLibrary.Array_IsNotEmpty` NavPts)
    (set `local.TmpNavPtsIn` (`local.NavPts`))
    (for _index (range _returnvalue (+ (`KismetStringLibrary.GetCharacterAsNumber` "Z") 1))
      (for _array_element _tmpnavptsin
        (if (`Actor.ActorHasTag` _array_element (`KismetStringLibrary.Conv_StringToName` (`|GetArrayItem` (`KismetStringLibrary.GetCharacterArrayFromString` "ABCDEFGHIJKLMNOPQRSTUVWXYZ") (- _index _returnvalue))))
          (`KismetArrayLibrary.Array_Add` (`local.TmpNavPts`) _array_element)
          (`KismetArrayLibrary.Array_RemoveItem` _tmpnavptsin _array_element)
          (break))))
    (if (`local.IsDescend`)
      (`KismetArrayLibrary.Array_Reverse` (`local.TmpNavPts`)))
    (return (`local.TmpNavPts`))
    (else
      (return NavPts))))