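; BP_Berge is a Blueprint that tracks its position along navigation points through a current and a target trigger sphere.
; SwitchSrcDstNavPt swaps the two spheres and flips the IsGoPrevNavPt flag to reverse the direction of travel.
; UpdNavPtFromNewOne shifts the target sphere into the current slot and takes a new point as the target.
; The event graph and construction script hold no logic, and neither function is called within this file.
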(fn `SwitchSrcDstNavPt`
  (locals (TmpNavPt :type "TriggerSphere Object Reference"))
  (set `local.TmpNavPt` (`self.CurrTriggerSphere`))
  (set `self.CurrTriggerSphere` (`self.TargetTriggerSphere`))
  (set `self.TargetTriggerSphere` (`local.TmpNavPt`))
  (set `self.IsGoPrevNavPt` (not (`self.IsGoPrevNavPt`))))

(fn `UpdNavPtFromNewOne`
  (params (NewNavPt :type "TriggerSphere Object Reference"))
  (set `self.CurrTriggerSphere` (`self.TargetTriggerSphere`))
  (set `self.TargetTriggerSphere` NewNavPt))

(fn `UserConstructionScript`)