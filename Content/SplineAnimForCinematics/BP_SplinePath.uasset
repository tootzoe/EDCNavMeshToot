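; Cinematic spline path actor that moves a referenced mesh actor along a spline while keeping it seated on the surface below.
; While IsRendering is set, each LiveLink controller update places a guide cube on the spline at the SplineAnim alpha and traces down from it.
; The mesh snaps to the hit point, taking pitch and roll from the surface normal and yaw from the spline, plus offsets.
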(event `self.LiveLinkComponentController.OnLiveLinkUpdated`
  (params (DeltaTime :type "Float (single-precision)"))
  (if (`self.IsRendering`)
    (`KismetSystemLibrary.PrintString` (`KismetStringLibrary.Conv_DoubleToString` (`self.SplineAnim`)) false false (struct :`G` 0.66 :`B` 1.0 :`A` 1.0) 2.0 "toot")
    (`self.SplineAnimator`)))

(fn `SplineAnimator`
  (bind (_returnvalue_roll _returnvalue_pitch _returnvalue_yaw) (`KismetMathLibrary.BreakRotator` (`self.K2_GetActorRotation`)))
  (bind _mainshowingactor (`self.MainShowingActor`))
  (bind (_returnvalue_roll_2 _returnvalue_pitch_2 _returnvalue_yaw_2) (`KismetMathLibrary.BreakRotator` (`SplineComponent.GetRotationAtTime` (`self.Spline`) (`self.SplineAnim`) "Local" true)))
  (bind (_returnvalue_x _returnvalue_y _returnvalue_z) (`KismetMathLibrary.BreakVector` (`SceneComponent.K2_GetComponentLocation` (`self.Cube`))))
  (`KismetArrayLibrary.Array_Set` (`self.ActorsToIgnore`) 0 (`self.MainShowingActor`))
  (set `self.SplineRotAtTime` (`SplineComponent.GetRotationAtTime` (`self.Spline`) (`self.SplineAnim`) "World" false))
  (`SceneComponent.K2_SetWorldLocationAndRotation` (`self.Cube`) (`SplineComponent.GetLocationAtDistanceAlongSpline` (`self.Spline`) (`KismetMathLibrary.Lerp` 0.0 (`SplineComponent.GetSplineLength` (`self.Spline`)) (`self.SplineAnim`)) "World") (`self.SplineRotAtTime`) false false)
  (bind _outhit (`KismetSystemLibrary.LineTraceSingleForObjects` (`KismetMathLibrary.MakeVector` _returnvalue_x _returnvalue_y (- _returnvalue_z 10.0)) (`KismetMathLibrary.MakeVector` _returnvalue_x _returnvalue_y -2000.0) (`self.SplineCubeTracingObjects`) false (`self.ActorsToIgnore`) "ForOneFrame" true (struct :`R` 1.0 :`A` 1.0) (struct :`G` 1.0 :`A` 1.0) 0.0))
  (set `self.RotZ_Offset` _returnvalue_yaw)
  (bind (_bblockinghit _binitialoverlap _time _distance _location _impactpoint _normal _impactnormal) (`GameplayStatics.BreakHitResult` _outhit))
  (bind _returnvalue_roll_3 (`KismetMathLibrary.BreakRotator` (`KismetMathLibrary.MakeRotFromXZ` (`self.GetActorForwardVector` _mainshowingactor) _impactnormal)))
  (bind (_returnvalue_roll_4 _returnvalue_pitch_3) (`KismetMathLibrary.BreakRotator` (`KismetMathLibrary.MakeRotFromYZ` (`self.GetActorRightVector` _mainshowingactor) _impactnormal)))
  (`SceneComponent.K2_SetWorldLocationAndRotation` (`StaticMeshActor.StaticMeshComponent` _mainshowingactor) _impactpoint (`KismetMathLibrary.MakeRotator` (+ _returnvalue_roll_3 (`self.RotX_Offset`)) (+ _returnvalue_pitch_3 (`self.RotY_Offset`)) (+ (`self.RotZ_Offset`) _returnvalue_yaw_2)) false false))

(fn `UserConstructionScript`)