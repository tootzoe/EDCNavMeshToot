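; BP_TestDynamicLink is a test actor that feeds a Live Link-driven custom direction into materials.
; On each Live Link update, it writes the vector from TestMesh to the actor's location, unnormalized, into the CustomDir parameter of the TootMPC material parameter collection.
; It also draws a debug arrow along that vector.
; An alternative write using the Arrow component's reversed forward vector is left disconnected.
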(event `self.LiveLinkComponentController.OnLiveLinkUpdated`
  (params (DeltaTime :type "Float (single-precision)"))
  (bind _returnvalue (`self.K2_GetActorLocation`))
  (bind _returnvalue_2 (`self.K2_GetActorLocation` (`self.TestMesh`)))
  (bind (_returnvalue_x _returnvalue_y _returnvalue_z) (`KismetMathLibrary.BreakVector` (- _returnvalue _returnvalue_2)))
  (`KismetMaterialLibrary.SetVectorParameterValue` (`self.TootMPC`) (`self.CustomDir`) (make `LinearColor` _returnvalue_x _returnvalue_y _returnvalue_z 1.0))
  (`KismetSystemLibrary.DrawDebugArrow` _returnvalue_2 (+ _returnvalue_2 (- _returnvalue _returnvalue_2)) 2222.0 (struct :`R` 1.0 :`B` 0.727163 :`A` 1.0) 0.0 3.0))

(fn `UserConstructionScript`)